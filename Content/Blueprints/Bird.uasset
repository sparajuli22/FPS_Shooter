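; Bird actor that wanders horizontally on its own, starting two seconds after play begins.
; A self-calling Move event chains two timed MoveComponentTo tweens: a random step toward negative X and Y, then one toward positive.
; The offsets are rolled independently from the current relative location, so the bird can drift, while height and rotation are carried over.
; MoveLeft and MoveRight helpers exist but are never executed.
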(event `self.ReceiveBeginPlay`
  (`KismetSystemLibrary.Delay` 2.0)
  (`self.Move`))

(event `Move`
  (bind _bird (`self.Bird`))
  (bind _bird_2 (`self.Bird`))
  ;[1 1 1] Movement
  (bind (_newpos _newrot) (`self.Move Random 1` _bird))
  (`KismetSystemLibrary.MoveComponentTo` _bird _newpos _newrot false false 1.0)
  (bind (_newpos_2 _newrot_2) (`self.Move Random 2` _bird_2))
  (`KismetSystemLibrary.MoveComponentTo` _bird_2 _newpos_2 _newrot_2 false false 1.0)
  (`self.Move`))

(fn `Move Left`
  (params (Mesh :type "StaticMeshComponent Object Reference"))
  (returns (newPos :type "Vector Structure") (newRot :type "Rotator Structure"))
  (bind (_relativelocation_x _relativelocation_y _relativelocation_z) (`KismetMathLibrary.BreakVector` (`SceneComponent.RelativeLocation` Mesh)))
  (return (`KismetMathLibrary.MakeVector` _relativelocation_x (- _relativelocation_y (`self.Movedistance`)) _relativelocation_z) (`SceneComponent.RelativeRotation` Mesh)))

(fn `Move Random 1`
  (params (NewParam :type "StaticMeshComponent Object Reference"))
  (returns (newPos :type "Vector Structure") (newRot :type "Rotator Structure"))
  (locals (NewLocalVar_0 :type "Vector Structure" :default (0.0 0.0 0.0)))
  (bind (_relativelocation_x _relativelocation_y _relativelocation_z) (`KismetMathLibrary.BreakVector` (`SceneComponent.RelativeLocation` NewParam)))
  (return (`KismetMathLibrary.MakeVector` (- _relativelocation_x (`KismetMathLibrary.RandomFloatInRange` 0.0 200.0)) (- _relativelocation_y (`KismetMathLibrary.RandomFloatInRange` 0.0 200.0)) _relativelocation_z) (`SceneComponent.RelativeRotation` NewParam)))

(fn `Move Random 2`
  (params (NewParam :type "StaticMeshComponent Object Reference"))
  (returns (newPos :type "Vector Structure") (newRot :type "Rotator Structure"))
  (locals (NewLocalVar_0 :type "Vector Structure" :default (0.0 0.0 0.0)))
  (bind (_relativelocation_x _relativelocation_y _relativelocation_z) (`KismetMathLibrary.BreakVector` (`SceneComponent.RelativeLocation` NewParam)))
  (return (`KismetMathLibrary.MakeVector` (+ (`KismetMathLibrary.RandomFloatInRange` 0.0 200.0) _relativelocation_x) (+ _relativelocation_y (`KismetMathLibrary.RandomFloatInRange` 0.0 200.0)) _relativelocation_z) (`SceneComponent.RelativeRotation` NewParam)))

(fn `Move Right`
  (params (Mesh :type "StaticMeshComponent Object Reference"))
  (returns (newPos :type "Vector Structure") (newRot :type "Rotator Structure"))
  (bind (_relativelocation_x _relativelocation_y _relativelocation_z) (`KismetMathLibrary.BreakVector` (`SceneComponent.RelativeLocation` Mesh)))
  (return (`KismetMathLibrary.MakeVector` _relativelocation_x (+ (`self.moveDIstance`) _relativelocation_y) _relativelocation_z) (`SceneComponent.RelativeRotation` Mesh)))

(fn `UserConstructionScript`)