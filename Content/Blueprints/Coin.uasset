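; Coin actor that destroys itself after a fixed delay from BeginPlay and has a Move event to animate its mesh.
; Move chains two timed MoveComponentTo calls, with targets from helpers that offset relative location by Movedistance: MoveLeft along negative Y, MoveRight along positive X.
; Only MoveRight's rotation is wired, so the second move targets the default relative location.
; Nothing in this Blueprint calls Move.
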(event `Move`
  (bind _coin (`self.coin`))
  (bind _coin_2 (`self.coin`))
  ;[1 1 1] Movement
  (bind (_newpos _newrot) (`self.Move Left` _coin_2))
  (`KismetSystemLibrary.MoveComponentTo` _coin_2 _newpos _newrot false false 2.0)
  (bind (_newpos_2 _newrot_2) (`self.Move Right` _coin))
  (`KismetSystemLibrary.MoveComponentTo` _coin (0.0 0.0 0.0) _newrot_2 false false 5.0))

(event `self.ReceiveBeginPlay`
  (`|ExecutionSequence`
    (:`then_0`
      (`KismetSystemLibrary.Delay` 10.0)
      (`self.K2_DestroyActor`))))

(fn `Move Left`
  (params (Mesh :type "StaticMeshComponent Object Reference"))
  (returns (newPos :type "Vector Structure") (newRot :type "Rotator Structure"))
  (bind (_relativelocation_x _relativelocation_y _relativelocation_z) (`KismetMathLibrary.BreakVector` (`SceneComponent.RelativeLocation` Mesh)))
  (return (`KismetMathLibrary.MakeVector` _relativelocation_x (- _relativelocation_y (`self.Movedistance`)) _relativelocation_z) (`SceneComponent.RelativeRotation` Mesh)))

(fn `Move Right`
  (params (Mesh :type "StaticMeshComponent Object Reference"))
  (returns (newPos :type "Vector Structure") (newRot :type "Rotator Structure"))
  (bind (_relativelocation_x _relativelocation_y _relativelocation_z) (`KismetMathLibrary.BreakVector` (`SceneComponent.RelativeLocation` Mesh)))
  (return (`KismetMathLibrary.MakeVector` (+ (`self.Movedistance`) _relativelocation_x) _relativelocation_y _relativelocation_z) (`SceneComponent.RelativeRotation` Mesh)))

(fn `UserConstructionScript`)